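; Character-logic Blueprint that tracks break-fall and crouch multi-tap input state, and resets global time dilation to normal on BeginPlay.
; SetBreakFall raises a BreakFall flag and clears it after a short retriggerable delay.
; The MultiTapInput macro counts calls with a counter that a retriggerable delay resets, returning true only for a single tap.
; CheckMultiTapInputCrouch inverts that result to flag repeated crouch taps within the window.
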(event `self.ReceiveBeginPlay`
  (`GameplayStatics.SetGlobalTimeDilation` 1.0))

(event `self.SetBreakFall`
  (set `self.BreakFall` true)
  (`KismetSystemLibrary.RetriggerableDelay` 0.4)
  (set `self.BreakFall` false))

(event `self.CheckMultiTapInputCrouch`
  (bind _issinglepress (`self.MultiTapInput` 0.3))
  (set `self.IsMultiTapInputCrouch` (not _issinglepress)))

(fn `UserConstructionScript`)